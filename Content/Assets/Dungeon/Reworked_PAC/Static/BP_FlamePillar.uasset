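; BP_FlamePillar is a dungeon flame pillar that makes its flame light flicker during play.
; From BeginPlay, it randomly picks one of two intensity timelines and picks again whenever one finishes, producing an endless, varied flicker loop.
; Each timeline update feeds ScaleFlameIntensity, which multiplies the curve value by BaseIntensity and applies it to FlameLight.
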(event Custom|Start_Timeline_1
  (bind _flameintensity (Timeline|FlameIntensityTimeline_1 PlayFromStart)
    (:Update
      (CallFunction|ScaleFlameIntensity _flameintensity))
    (:Finished
      (CallFunction|ChooseFlameLightTimeline))))

(event Custom|Start_Timeline_2
  (bind _flameintensity (Timeline|FlameIntensityTimeline_2 PlayFromStart)
    (:Update
      (CallFunction|ScaleFlameIntensity _flameintensity))
    (:Finished
      (CallFunction|ChooseFlameLightTimeline))))

(event Custom|ChooseFlameLightTimeline
  (switch int (Math|Random|RandomIntegerinRange 0 1)
    (:Default
      (CallFunction|StartTimeline2 :!label _label))
    (:0
      (CallFunction|StartTimeline1))
    (:1
      (goto _label))))

(event EventBeginPlay
  (CallFunction|ChooseFlameLightTimeline))

(fn ConstructionScript)

(fn ScaleFlameIntensity
  (params (Intensity :type Float%20%28double-precision%29))
  (Rendering|Components|Light|SetIntensity (Variables|Default|GetFlameLight) (* Intensity (Variables|Default|GetBaseIntensity))))