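; Base actor for meshes that fade out and back in, ignoring Visibility and a custom trace channel while faded.
; Construction caches original materials and builds dynamic instances from dedicated fade materials.
; FadeOut swaps these in and plays a timeline driving their "Fade" parameter, limited by FadeThreshold.
; FadeIn restores the saved collision profile immediately and reverses the timeline, which restores original materials once fully opaque.
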(event EventFadein
  (CallFunction|ResetCollisionProfile)
  (bind _fade (Timeline|FadeTimeline Reverse)
    (:Update
      (for _array_element (Variables|Default|GetDynamicMaterialsInstances)
        (Rendering|Material|SetScalarParameterValue _array_element "Fade" (Math|Float|Lerp (Variables|Default|GetFadeThreshold) 1.0 _fade) :!class /Script/Engine.MaterialInstanceDynamic)))
    (:Finished
      ;[1 1 1] When fully faded back in, set all of the Materials back to their original defaults and make the Mesh block the Visibility channel
      (if (>= (Math|Float|Lerp (Variables|Default|GetFadeThreshold) 1.0 _fade) 1.0)
        (CallFunction|ResetMaterialstoDefaults)))))

(event EventBeginPlay
  (Variables|Default|SetOriginalCollisionProfile (Collision|GetCollisionProfileName (Variables|Default|GetMesh))))

(event EventFadeOut
  (CallFunction|DisableCollisionResponses)
  (CallFunction|SetMaterialstoDynamicInstances)
  (bind _fade (Timeline|FadeTimeline Play)
    (:Update
      (for _array_element (Variables|Default|GetDynamicMaterialsInstances)
        (Rendering|Material|SetScalarParameterValue _array_element "Fade" (Math|Float|Lerp (Variables|Default|GetFadeThreshold) 1.0 _fade) :!class /Script/Engine.MaterialInstanceDynamic)))
    (:Finished
      ;[1 1 1] When fully faded back in, set all of the Materials back to their original defaults and make the Mesh block the Visibility channel
      (if (>= (Math|Float|Lerp (Variables|Default|GetFadeThreshold) 1.0 _fade) 1.0)
        (CallFunction|ResetMaterialstoDefaults)))))

(fn ConstructionScript
  (Utilities|Array|Clear (Variables|Default|GetDynamicMaterialsInstances))
  (Variables|Default|SetOriginalMaterials (Rendering|Material|GetMaterials (Variables|Default|GetMesh)))
  ;[1 1 1] Creates a Dynamic Material Instance from each of our Fade Material Instances
  (for _array_element (Variables|Default|GetFadeMaterialInstances)
    (bind _returnvalue (Rendering|Material|CreateDynamicMaterialInstance _array_element "None" "None" :!class /Script/Engine.KismetMaterialLibrary))
    (Utilities|Array|AddUnique (Variables|Default|GetDynamicMaterialsInstances) _returnvalue)))

(fn SetMaterialstoDynamicInstances
  (for (_array_element _array_index) (Variables|Default|GetDynamicMaterialsInstances)
    (Rendering|Material|SetMaterial (Variables|Default|GetMesh) _array_index _array_element)))

(fn ResetMaterialstoDefaults
  (for (_array_element _array_index) (Variables|Default|GetOriginalMaterials)
    (Rendering|Material|SetMaterial (Variables|Default|GetMesh) _array_index _array_element)))

(fn DisableCollisionResponses
  (Collision|SetCollisionResponsetoChannel (Variables|Default|GetMesh) "ECC_Visibility" "ECR_Ignore")
  (Collision|SetCollisionResponsetoChannel (Variables|Default|GetMesh) "ECC_GameTraceChannel2" "ECR_Ignore"))

(fn ResetCollisionProfile
  (Collision|SetCollisionProfileName (Variables|Default|GetMesh) (Variables|Default|GetOriginalCollisionProfile) true :!class /Script/Engine.PrimitiveComponent))