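; BP_PlayerCharacter is the player character Blueprint, handling camera-occlusion fading, a motion-warp facing target and a shock-loop flag.
; While the locally controlled character moves, CameraFadeOutHeper overlaps send fade-out and fade-in messages to actors implementing BPI_FadeInterface.
; Events update the "FacingTarget" warp location in MotionWarping and set InShockLoop.
; IsMoving treats any non-zero CharacterMovement velocity as movement, gating both fade messages.
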(event OnComponentBeginOverlap(CameraFadeOutHeper)
  (params (OverlappedComponent :type Primitive%20Component%20Object%20Reference) (OtherActor :type Actor%20Object%20Reference) (OtherComp :type Primitive%20Component%20Object%20Reference) (OtherBodyIndex :type Integer) (bFromSweep :type Boolean) (SweepResult :type Hit%20Result%20Structure%20%28by%20ref%29))
  (if (Pawn|IsLocallyControlled)
    (bind _moving (CallFunction|IsMoving))
    (if _moving
      (if (Utilities|DoesObjectImplementInterface OtherActor "/Game/Assets/Dungeon/Reworked_PAC/FadeActors/Core/BPI_FadeInterface.BPI_FadeInterface_C")
        (Class|BPIFadeInterface|FadeOut(Message) OtherActor)))))

(event OnComponentEndOverlap(CameraFadeOutHeper)
  (params (OverlappedComponent :type Primitive%20Component%20Object%20Reference) (OtherActor :type Actor%20Object%20Reference) (OtherComp :type Primitive%20Component%20Object%20Reference) (OtherBodyIndex :type Integer))
  (if (Pawn|IsLocallyControlled)
    (bind _moving (CallFunction|IsMoving))
    (if _moving
      (if (Utilities|DoesObjectImplementInterface OtherActor "/Game/Assets/Dungeon/Reworked_PAC/FadeActors/Core/BPI_FadeInterface.BPI_FadeInterface_C")
        (Class|BPIFadeInterface|Fadein(Message) OtherActor)))))

(event EventUpdateFacingTarget
  (params (Target :type Vector%20%28by%20ref%29 :default "0, 0, 0"))
  (Class|MotionWarpingComponent|AddorUpdateWarpTargetfromLocation (Variables|Default|GetMotionWarping) "FacingTarget" Target))

(event EventSetinShockLoop
  (params (bInLoop :type Boolean))
  (Variables|Default|SetInShockLoop bInLoop))

(fn ConstructionScript)

(fn IsMoving
  (return (> (Math|Vector|VectorLength (Variables|/Script/Engine.MovementComponent|GetVelocity (Variables|Character|GetCharacterMovement))) 0.0)))