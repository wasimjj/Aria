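; Base Blueprint for enemy characters that handles attack-facing and the dissolve visuals for body and weapon.
; UpdateFacingTarget feeds a location into the Motion Warping "FacingTarget" warp target.
; Each dissolve event waits half the remaining TTL, applies the supplied dynamic material instance to the mesh or weapon, then drives its "Dissolve" parameter from a timeline.
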(event EventUpdateFacingTarget
  (params (Target :type Vector%20%28by%20ref%29 :default "0, 0, 0"))
  (Class|MotionWarpingComponent|AddorUpdateWarpTargetfromLocation (Variables|Default|GetMotionWarping) "FacingTarget" Target))

(event EventStartWeaponDissolveTimeline
  (params (WeaponDynamicMaterialInstance :type Material%20Instance%20Dynamic%20Object%20Reference))
  (bind _returnvalue (Class|CombatInterface|GetRemainingTTL))
  (Utilities|FlowControl|Delay (/ _returnvalue 2.0))
  (Rendering|Material|SetMaterial (Variables|Default|GetWeapon) 0 WeaponDynamicMaterialInstance)
  (Utilities|IsValid WeaponDynamicMaterialInstance
    (:Is%20Valid
      (bind _weapondissolvetrack (Timeline|WeaponDissolveTimeline PlayFromStart)
        (:Update
          (Rendering|Material|SetScalarParameterValue WeaponDynamicMaterialInstance "Dissolve" _weapondissolvetrack :!class /Script/Engine.MaterialInstanceDynamic))))))

(event EventStartDissolveTimeline
  (params (DynamicMaterialInstance :type Material%20Instance%20Dynamic%20Object%20Reference))
  (bind _returnvalue (Class|CombatInterface|GetRemainingTTL))
  (Utilities|FlowControl|Delay (/ _returnvalue 2.0))
  (Rendering|Material|SetMaterial (Variables|Character|GetMesh) 0 DynamicMaterialInstance)
  (Utilities|IsValid DynamicMaterialInstance
    (:Is%20Valid
      (bind _dissolvetrack (Timeline|DissolveTimeline PlayFromStart)
        (:Update
          (Rendering|Material|SetScalarParameterValue DynamicMaterialInstance "Dissolve" _dissolvetrack :!class /Script/Engine.MaterialInstanceDynamic))))))

(fn ConstructionScript)