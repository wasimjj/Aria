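; Gameplay Ability that makes its avatar face the combat target and summon random minions around itself.
; The summoning montage's gameplay event starts a timed radial point generation on the ground, whose per-point callback spawns VFX and a minion while the owner's count is below the limit.
; Minions face the target, get a controller and register their owner through interface messages.
; The ability ends on point completion or montage interruption; older spawn-loop logic remains disconnected.
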(event Ability|EventActivateAbility
  (bind _returnvalue (Ability|GetAvatarActorfromActorInfo))
  (CallFunction|EnforceImplementsCombatInterface)
  (bind _returnvalue_2 (Class|CombatInterface|GetCombatTarget(Message) (Ability|GetAvatarActorfromActorInfo)))
  (Variables|Default|SetFacingTarget (Transformation|GetActorLocation _returnvalue_2))
  (CallFunction|UpdateFacingTarget)
  (|PlayMontageandWaitProxy "None" "/Game/Assets/Characters/Enemies/Shaman/Animations/AM_Summoning_GoblinShamon.AM_Summoning_GoblinShamon" 1.0 "None" true 1.0 0.0 false
    (:then
      (Ability|Tasks|WaitGameplayEvent "(TagName=\"Montage.Summoning\")" 0 true
        (:EventReceived
          (|GeneratePointArray (Transformation|GetActorLocation _returnvalue) (Transformation|GetActorForwardVector _returnvalue) "Radial" (Variables|Default|GetNumMinionsToSummon) 0.1 "Random" 2e+02 (Math|Vector|VectorUp) 0.0 false "175.f" "175.f" true 0.0 0.0 0.0 0.0 false false false false false false))))
    (:OnInterrupted
      ;[1 1 1] This prevents the Animation from becoming locked up when the Summon Ability gets interrupted.
      (Ability|EndAbility :!label _label))
    (:OnCancelled
      (goto _label))))

(event EventOnArrayPointCreatedBP
  (params (NewPoint :type Gyro%20Axis%20Point%20Structure%20%28by%20ref%29))
  (bind _returnvalue (Class|CombatInterface|GetMinionCount(Message) (Ability|GetAvatarActorfromActorInfo)))
  (if (< _returnvalue (Variables|Default|GetNumMinionsToSummon))
    (Class|CombatInterface|IncrementMinionCount(Message) (Ability|GetAvatarActorfromActorInfo) 1)
    (bind _output_get (Variables|Default|SetSpawnLocation (.Position (Utilities|Struct|BreakGyroAxisPoint NewPoint))))
    (Niagara|SpawnSystematLocation (Variables|Default|GetMinionPreSummonVFX) _output_get)
    (Niagara|SpawnSystematLocation (Variables|Default|GetMinionPostSummonVFX) (Variables|Default|GetSpawnLocation))
    (CallFunction|SpawnMinion (Variables|Default|GetSpawnLocation))))

(event EventOnPointArrayCompletedBP
  (Ability|EndAbility))

(fn SpawnMinion
  (params (SpawnLocation :type Vector))
  (bind _returnvalue (+ SpawnLocation "0.000000,0.000000,70.000000"))
  (bind _returnvalue_2 (Game|SpawnActorfromClass (Class|AriaSummonAbility|GetRandomMinionClass) (Math|Transform|MakeTransform _returnvalue (Math|Rotator|FindLookatRotation _returnvalue (Variables|Default|GetFacingTarget)) "1.000000,1.000000,1.000000") "Undefined" "MultiplyWithRoot" 0 0))
  (bind _output_get (LocalVariables|SetSpawnedActor _returnvalue_2))
  (Pawn|SpawnDefaultController _output_get)
  (Class|CombatInterface|SetCharacterasMinion(Message) (LocalVariables|GetSpawnedActor))
  (Class|CombatInterface|SetMinionOwningCharacter(Message) (LocalVariables|GetSpawnedActor) (Ability|GetAvatarActorfromActorInfo))
  (LocalVariables|SetOwnerActor (Ability|GetAvatarActorfromActorInfo))
  (return))

(fn EnforceImplementsCombatInterface
  ;[1 0.6096 0] Verify Implements the Combat Interface
  (if (not (Utilities|DoesObjectImplementInterface (Ability|GetAvatarActorfromActorInfo) "/Script/Aria.CombatInterface"))
    (Ability|EndAbility)))

(fn UpdateFacingTarget
  (Class|CombatInterface|UpdateFacingTarget(Message) (Ability|GetAvatarActorfromActorInfo) (Variables|Default|GetFacingTarget)))