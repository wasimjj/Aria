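; Firebolt gameplay ability that casts fire projectiles from the avatar's weapon socket toward the point or actor under the mouse.
; On a blocking cursor hit it commits, turns the avatar to face the target through CombatInterface and plays the cast montage.
; A montage gameplay event triggers SpawnProjectile, passing the hit actor as homing target.
; The ability ends without a blocking hit or when the montage finishes or is interrupted.
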(event Ability|EventActivateAbility
  (CallFunction|EnforceImplementsCombatInterface)
  (bind _datahandle (|TargetDataUnderMouse)
    (:ValidData
      (if (.bBlockingHit (Collision|BreakHitResult (Ability|TargetData|GetHitResultfromTargetData _datahandle)))
        (Ability|CommitAbility)
        (Variables|Default|SetProjectileTargetLocation (.Location (Collision|BreakHitResult (Ability|TargetData|GetHitResultfromTargetData _datahandle))))
        (Variables|Default|SetCursorHitActor (.HitActor (Collision|BreakHitResult (Ability|TargetData|GetHitResultfromTargetData _datahandle))))
        (CallFunction|UpdateFacingTarget)
        (|PlayMontageandWaitProxy "None" "/Game/Assets/Characters/Aura/Animations/Abilities/AM_Cast_Firebolt.AM_Cast_Firebolt" 1.0 "None" false 1.0 0.0 false
          (:then
            (Ability|Tasks|WaitGameplayEvent "(TagName=\"Event.Montage.Firebolt\")" 0 true
              (:EventReceived
                (bind _returnvalue (Class|CombatInterface|GetCombatSocketLocation(Message) (Ability|GetAvatarActorfromActorInfo) (GameplayTags|MakeLiteralGameplayTag "(TagName=\"CombatSocket.Weapon\")")))
                (Variables|Default|SetProjectileDirection (Transformation|GetActorForwardVector (Ability|GetAvatarActorfromActorInfo)))
                (Class|AriaProjectileAbility|SpawnProjectile :ProjectileTargetLocation (Variables|Default|GetProjectileTargetLocation) :ForwardFacingVector (Variables|Default|GetProjectileDirection) :GyroAxisPoint (Utilities|Struct|MakeGyroAxisPoint _returnvalue "0.000000,0.000000,0.000000") :HomingTarget (Variables|Default|GetCursorHitActor)))))
          (:OnCompleted
            (Ability|EndAbility :!label _label))
          (:OnBlendOut
            (goto _label))
          (:OnInterrupted
            (goto _label))
          (:OnCancelled
            (goto _label)))
        (else
          (Ability|EndAbility))))))

(fn EnforceImplementsCombatInterface
  ;[1 0.6096 0] Verify Implements the Combat Interface
  (if (not (Utilities|DoesObjectImplementInterface (Ability|GetAvatarActorfromActorInfo) "/Script/Aria.CombatInterface"))
    (Ability|EndAbility)))

(fn UpdateFacingTarget
  (Class|CombatInterface|UpdateFacingTarget(Message) (Ability|GetAvatarActorfromActorInfo) (Variables|Default|GetProjectileTargetLocation)))