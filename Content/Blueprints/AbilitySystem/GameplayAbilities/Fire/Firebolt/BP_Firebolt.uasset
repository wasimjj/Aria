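; Firebolt projectile actor for the fire gameplay ability.
; On BeginPlay it waits briefly before switching its Sphere to query-only collision on a custom trace channel object type.
; Every Tick it compares its position with the previous frame's, and if movement falls to a minimum threshold or below, it treats itself as stuck, plays impact sound and Niagara explosion, then destroys itself.
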(event EventBeginPlay
  (Utilities|FlowControl|Delay 0.1)
  (bind _sphere (Variables|Default|GetSphere)
    (:then
      (Collision|SetCollisionEnabled _sphere "QueryOnly")
      (Collision|SetCollisionObjectType (Variables|Default|GetSphere) "ECC_GameTraceChannel1"))
    (:else)))

(event EventTick
  (params (DeltaSeconds :type Float%20%28single-precision%29))
  (CallFunction|ForceDestroyifStuck))

(fn ConstructionScript)

(fn ForceDestroyifStuck
  (Variables|Default|SetLocationLastFrame (Variables|Default|GetLocationThisFrame))
  (Variables|Default|SetLocationThisFrame (Transformation|GetActorLocation))
  ;[1 0.185 0] Check Whether the Projectile is Moving faster than the MinDistancePerFrame threshold;
  ; If  not, then Destroy the Projectile
  (if (<= (Math|Vector|VectorLength (- (Variables|Default|GetLocationThisFrame) (Variables|Default|GetLocationLastFrame))) (Variables|Default|GetMinDistancePerFrame))
    (Audio|SpawnSoundatLocation "/Game/Assets/Sounds/Abilities/FireBolt/sfx_FireBolt_Impact.sfx_FireBolt_Impact" (Variables|Default|GetLocationThisFrame) "0, 0, 0" 1.0 1.0 0.0 0 0)
    (Niagara|SpawnSystematLocation "/Game/Assets/Effects/Stylized/Explosion/NS_Stylized_FireExplosion.NS_Stylized_FireExplosion" (Variables|Default|GetLocationThisFrame))
    (Actor|DestroyActor)))