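; GA_Storm is a gameplay ability that casts a lightning storm at a point the player picks with an AoE targeting reticle.
; An input press captures the mouse target, turns the avatar toward it, starts the storm sound and plays the cast montage.
; The montage event starts randomly sequenced, ground-snapped point generation, then the ability ends after a brief delay.
; Each point fires the Storm gameplay cue, and completion fades the sound.
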(event Ability|EventActivateAbility
  (Utilities|FlowControl|Sequence
    (:then_0
      (Class|TargetingInterface|ShowAoETargetingReticle(Message) (Ability|GetAvatarActorfromActorInfo) "/Game/Assets/Materials/MagicCircles/MI_MagicCircle_Blue.MI_MagicCircle_Blue" (Variables|Default|GetTargetingAreaRadius)))
    (:then_1
      (Ability|Tasks|WaitInputPress false
        (:OnPress
          (bind _datahandle (|TargetDataUnderMouse)
            (:ValidData
              (Variables|Default|SetImpactPoint (.ImpactPoint (Collision|BreakHitResult (Ability|TargetData|GetHitResultfromTargetData _datahandle))))
              (Class|TargetingInterface|HideAoETargetingReticle(Message) (Ability|GetAvatarActorfromActorInfo))
              (CallFunction|EnforceImplementsCombatInterface)
              (CallFunction|UpdateFacingTarget)
              (Utilities|FlowControl|Sequence
                (:then_0
                  (bind _returnvalue (Audio|SpawnSoundatLocation "/Game/Assets/Sounds/Abilities/Storm/sfx_IncomingStorm.sfx_IncomingStorm" (Variables|Default|GetImpactPoint) "0, 0, 0" 1.0 1.0 0.0 0 0))
                  (Variables|Default|SetStormSound _returnvalue))
                (:then_1
                  (|PlayMontageandWaitProxy "None" "/Game/Assets/Characters/Aura/Animations/Abilities/AM_Cast_Storm.AM_Cast_Storm" 1.0 "None" false 1.0 0.0 false
                    (:then
                      (Ability|Tasks|WaitGameplayEvent "(TagName=\"Event.Montage.Storm\")" 0 true
                        (:EventReceived
                          (|GeneratePointArray (Variables|Default|GetImpactPoint) "No_Pattern" 25 0.2 "Random" "150.f" true 0.0 0.0 0.0 0.0 false false false false false)
                          (Utilities|FlowControl|Delay 0.2)
                          (Ability|EndAbility))))))))))))))

(event EventOnArrayPointCreatedBP
  (params (NewPoint :type Gyro%20Axis%20Point%20Structure%20%28by%20ref%29))
  (Class|GameplayAbility|ExecuteGameplayCuewithParams "(TagName=\"GameplayCue.Storm\")" (Ability|GameplayCue|MakeGameplayCueParameters :Location (.Position (Utilities|Struct|BreakGyroAxisPoint NewPoint)))))

(event EventOnPointArrayCompletedBP
  (bind _stormsound (Variables|Default|GetStormSound)
    (:then
      (Audio|Components|Audio|FadeOut _stormsound 2.5 0.0 "Linear" :!class /Script/Engine.AudioComponent))
    (:else)))

(fn UpdateFacingTarget
  (Class|CombatInterface|UpdateFacingTarget(Message) (Ability|GetAvatarActorfromActorInfo) (Variables|Default|GetImpactPoint)))

(fn EnforceImplementsCombatInterface
  ;[1 0.6096 0] Verify Implements the Combat Interface
  (if (not (Utilities|DoesObjectImplementInterface (Ability|GetAvatarActorfromActorInfo) "/Script/Aria.CombatInterface"))
    (Ability|EndAbility)))