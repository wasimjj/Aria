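; GA_Shock is a held lightning beam ability that shocks the cursor target and additional targets, locking caster movement while active.
; A montage event starts the ShockLoop gameplay cues, chained from weapon to first target to the others, and a looping timer that commits cost and applies damage on authority.
; Release after a minimum hold, insufficient cost, or primary target death ends it, applying final damage and committing cooldown.
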(event Custom|SetDamageAndCost
  (bind _returnvalue (Ability|CommitAbilityCost false))
  (if _returnvalue
    (Ability|HasAuthority
      (:True
        (CallFunction|ApplyDamagetoAllTargets)))
    (else
      ;[0.03412 1 0] Not Enough Mana Left... End the Ability.
      (CallFunction|ClearTimerandEndAbility))))

(event Ability|EventActivateAbility
  (CallFunction|EnforceImplementsCombatInterface)
  ;[1 1 1] Store Mouse Location / Target Data
  (bind _datahandle (|TargetDataUnderMouse)
    (:ValidData
      (Class|AriaShockAbility|StoreCursorDataInfo (Ability|TargetData|GetHitResultfromTargetData _datahandle))
      (Class|AriaShockAbility|StoreOwnerVariables)
      (Utilities|FlowControl|Sequence
        (:then_0
          (CallFunction|HideMouseCursor)
          (CallFunction|UpdateFacingTarget)
          (GameplayCue|ExecuteGameplayCue :GameplayCueTag "(TagName=\"GameplayCue.ShockBurst\")")
          (|PlayMontageandWaitProxy "None" (Variables|Default|GetMontage_Shock) 1.0 "None" true 1.0 0.0 false
            (:then
              (Ability|Tasks|WaitGameplayEvent "(TagName=\"Event.Montage.Shock\")" 0 true
                (:EventReceived
                  (CallFunction|InShockLoop)
                  (bind _returnvalue (Utilities|Time|SetTimerbyEvent (delegate Custom|SetDamageAndCost) (Variables|Default|GetDamageDeltaTime) true))
                  (Variables|Default|SetDamageAndCostTimer _returnvalue))))))
        (:then_1
          (bind _timeheld (Ability|Tasks|WaitInputRelease false)
            (:OnRelease
              ;[1 0.425 0] Check if the Minimum Ability Active Time has been reached; if not then delay the Ability for the length of time required (ex: 0.5 seconds)
              ;   Note: This will force the Ability to always Activate even if only for a brief second (i.e. Enforces the Minimum Ability Activation Time)
              (Variables|Default|SetInputTimeHeld _timeheld)
              (if (< (Variables|Default|GetInputTimeHeld) (Variables|Default|GetMinInputHoldTime))
                (Ability|HasAuthority
                  (:True
                    (Utilities|FlowControl|Delay (- (Variables|Default|GetMinInputHoldTime) (Variables|Default|GetInputTimeHeld)))
                    (CallFunction|ClearTimerandEndAbility :!label _label))
                  (:False
                    (CallFunction|PreparetoEndAbility)))
                (else
                  (goto _label))))))))))

(event EventPrimaryTargetDied
  (params (DeadActor :type Actor%20Object%20Reference))
  ;[0 0.4313 1] Primary target Died
  (GameplayCue|RemoveGameplayCueOnActor(Looping) :Target DeadActor :Parameters (Variables|Default|GetFirstTargetCueParams))
  (CallFunction|ClearTimerandEndAbility))

(event EventAdditionalTargetDied
  (params (DeadActor :type Actor%20Object%20Reference))
  ;[0.2718 0 1] Additional Target Died (Remove from Additional Targets and Remove from ShockLoop Queue)
  (CallFunction|RemoveShockLoopCuefromTarget DeadActor)
  (Utilities|Array|RemoveItem (Variables|Default|GetAdditionalTargets) DeadActor))

(fn EnforceImplementsCombatInterface
  ;[1 0.6096 0] Verify Implements the Combat Interface
  (if (not (Utilities|DoesObjectImplementInterface (Ability|GetAvatarActorfromActorInfo) "/Script/Aria.CombatInterface"))
    (Ability|EndAbility)))

(fn HideMouseCursor
  ;[1 1 1] Hide the Mouse Cursor when Activating the Ability
  (Variables|/Script/Engine.PlayerController|SetbShowMouseCursor (Variables|Default|GetOwnerPlayerController) false))

(fn ShowMouseCursor
  ;[1 1 1] Show the Mouse Cursor after Deactivating the Ability
  (Variables|/Script/Engine.PlayerController|SetbShowMouseCursor (Variables|Default|GetOwnerPlayerController) true))

(fn UpdateFacingTarget
  (Class|CombatInterface|UpdateFacingTarget(Message) (Ability|GetAvatarActorfromActorInfo) (Variables|Default|GetCursorHitLocation)))

(fn InShockLoop
  (Class|CombatInterface|SetinShockLoop(Message) (Ability|GetAvatarActorfromActorInfo) true)
  ;[1 1 1] Disabling Character Movements while the Ability is Active
  (Pawn|Components|CharacterMovement|DisableMovement (Variables|/Script/Engine.Character|GetCharacterMovement (Variables|Default|GetOwnerCharacter)))
  (CallFunction|SpawnShockSystem))

(fn SpawnShockSystem
  (Class|AriaShockAbility|TraceFirstTarget (Variables|Default|GetCursorHitLocation))
  (bind _returnvalue (Class|CombatInterface|GetWeapon(Message) (Variables|Default|GetOwnerCharacter)))
  (Variables|Default|SetFirstTargetCueParams (Ability|GameplayCue|MakeGameplayCueParameters :Location (Variables|Default|GetCursorHitLocation) :SourceObject (Variables|Default|GetCursorHitActor) :TargetAttachComponent _returnvalue))
  ;[1 1 1] Does Cursor Hit Actor implement Combat Interface;
  ; This verifies whether hitting a Character (like an Enemy/ or NPC) or hitting just a geometry object such as a Wall or Floor
  (bind _output_get (Variables|Default|SetFirstTargetImpInterface (Utilities|DoesObjectImplementInterface (Variables|Default|GetCursorHitActor) "/Script/Aria.CombatInterface")))
  (if _output_get
    (Variables|Default|SetCueTarget (Variables|Default|GetCursorHitActor))
    (else
      (Variables|Default|SetCueTarget (Ability|GetAvatarActorfromActorInfo))))
  (GameplayCue|AddGameplayCueOnActor(Looping) (Variables|Default|GetCueTarget) "(TagName=\"GameplayCue.ShockLoop\")" (Variables|Default|GetFirstTargetCueParams))
  ;[1 0 0.9215] Only Add the Additional Gameplay Cues if hit a Target that implements Combat Interface
  (if (Variables|Default|GetFirstTargetImpInterface)
    ;[0 1 0.203] Set Is Being Shocked on first Character; Handles triggering the Character Shock Animation
    (Class|CombatInterface|SetIsBeingShocked(Message) (Variables|Default|GetCueTarget) true)
    (bind _outadditionaltargets (Class|AriaShockAbility|StoreAdditionalTargets))
    (bind _output_get_2 (Variables|Default|SetAdditionalTargets _outadditionaltargets))
    (for _array_element _output_get_2
      (CallFunction|AddShockLoopCuetoTarget _array_element)
      ;[0 1 0.203] Set Is Being Shocked for each additional Character
      (Class|CombatInterface|SetIsBeingShocked(Message) _array_element true))))

(fn PreparetoEndAbility
  (Class|CombatInterface|SetinShockLoop(Message) (Ability|GetAvatarActorfromActorInfo) false)
  ;[1 1 1] Reenabling Character Movement after Deactivating the Ability
  (Pawn|Components|CharacterMovement|SetMovementMode (Variables|/Script/Engine.Character|GetCharacterMovement (Variables|Default|GetOwnerCharacter)) "MOVE_Walking" 0)
  (CallFunction|ShowMouseCursor)
  (if (Variables|Default|GetFirstTargetImpInterface)
    (GameplayCue|RemoveGameplayCueOnActor(Looping) (Variables|Default|GetCursorHitActor) "(TagName=\"GameplayCue.ShockLoop\")" (Variables|Default|GetFirstTargetCueParams))
    ;[0 1 0.203] Set Is Being Shocked on first Character to false; Handles stopping the Character Shock Animation
    (Class|CombatInterface|SetIsBeingShocked(Message) (Variables|Default|GetCursorHitActor) false)
    ;[1 0 0.3309] Apply Final Damage Effect to First Target
    (Ability|HasAuthority
      (:True
        (Class|AriaAbilitySystemLibrary|ApplyDamageEffect (Class|AriaDamageGameplayAbility|MakeFinalAbilityModifierfromClassDefaults (Variables|Default|GetCursorHitActor))))
      (:False
        _))
    ;[1 1 1] Remove Gameplay Cue from Each Additional Target
    (for _array_element (Variables|Default|GetAdditionalTargets)
      (CallFunction|RemoveShockLoopCuefromTarget _array_element)
      ;[0 1 0.203] Set Is Being Shocked to false for each additional Character
      (Class|CombatInterface|SetIsBeingShocked(Message) _array_element false)
      ;[1 0 0.3309] Apply Final Damage Effect to Each Additional Target
      (Ability|HasAuthority
        (:True
          (Class|AriaAbilitySystemLibrary|ApplyDamageEffect (Class|AriaDamageGameplayAbility|MakeFinalAbilityModifierfromClassDefaults _array_element)))))
    (else
      ;[1 1 1] Probably was just a Wall, Floor, etc.
      (GameplayCue|RemoveGameplayCueOnActor(Looping) (Ability|GetAvatarActorfromActorInfo) "(TagName=\"GameplayCue.ShockLoop\")" (Variables|Default|GetFirstTargetCueParams)))))

(fn ClearTimerandEndAbility
  (Utilities|Time|ClearandInvalidateTimerbyHandle (Variables|Default|GetDamageAndCostTimer))
  (CallFunction|PreparetoEndAbility)
  (Ability|CommitAbilityCooldown false)
  ;[1 0 0.4514] Garbage Collection
  (Utilities|Array|Clear (Variables|Default|GetAdditionalTargets))
  (Utilities|Map|Clear (Variables|Default|GetAdditionalActorsToCueParams))
  (Variables|Default|SetCursorHitActor 0)
  (Variables|Default|SetFirstTargetImpInterface false)
  (Variables|Default|SetInputTimeHeld 0.0)
  (Ability|EndAbility))

(fn AddShockLoopCuetoTarget
  (params (Target :type Actor%20Object%20Reference))
  (LocalVariables|SetTargetActor Target)
  (Utilities|Map|Add (Variables|Default|GetAdditionalActorsToCueParams) (LocalVariables|GetTargetActor) (Ability|GameplayCue|MakeGameplayCueParameters :Location (Transformation|GetActorLocation (LocalVariables|GetTargetActor)) :SourceObject (LocalVariables|GetTargetActor) :TargetAttachComponent (Variables|/Script/Engine.Actor|GetRootComponent (Variables|Default|GetCursorHitActor))))
  (GameplayCue|AddGameplayCueOnActor(Looping) (LocalVariables|GetTargetActor) "(TagName=\"GameplayCue.ShockLoop\")" (Ability|GameplayCue|MakeGameplayCueParameters :Location (Transformation|GetActorLocation (LocalVariables|GetTargetActor)) :SourceObject (LocalVariables|GetTargetActor) :TargetAttachComponent (Variables|/Script/Engine.Actor|GetRootComponent (Variables|Default|GetCursorHitActor)))))

(fn RemoveShockLoopCuefromTarget
  (params (Target :type Actor%20Object%20Reference))
  (bind _additionalactorstocueparams (Variables|Default|GetAdditionalActorsToCueParams))
  (bind (_value _returnvalue) (Utilities|Map|Find _additionalactorstocueparams Target))
  (if _returnvalue
    (GameplayCue|RemoveGameplayCueOnActor(Looping) Target "(TagName=\"GameplayCue.ShockLoop\")" _value)))

(fn ApplyDamageEffecttoTarget
  (params (Target :type Actor%20Object%20Reference))
  (bind _output_get (LocalVariables|SetDamageTarget Target))
  (Utilities|IsValid _output_get
    (:Is%20Valid
      (bind _output_get_2 (LocalVariables|SetTargetASC (Ability|GetAbilitySystemComponent (LocalVariables|GetDamageTarget))))
      (Utilities|IsValid _output_get_2
        (:Is%20Valid
          (Ability|HasAuthority
            (:True
              (Class|AriaAbilitySystemLibrary|ApplyDamageEffect (Class|AriaDamageGameplayAbility|MakeAbilityModifierfromClassDefaults (LocalVariables|GetDamageTarget))))))))))

(fn ApplyDamagetoAllTargets
  (CallFunction|ApplyDamageEffecttoTarget (Variables|Default|GetCursorHitActor))
  (for _array_element (Variables|Default|GetAdditionalTargets)
    (CallFunction|ApplyDamageEffecttoTarget _array_element)))