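; Gameplay ability for an enemy ranged attack that turns the avatar toward its combat target and plays a random attack montage.
; The montage's gameplay event triggers caching of the combat socket location and forward vector as projectile inputs.
; SpawnProjectile is left unconnected, so this graph fires no projectile itself.
; Montage completion, interruption or cancellation ends the ability, preventing locked-up animation after interrupted attacks.
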(event Ability|EventActivateAbility
  (bind _returnvalue (Ability|GetAvatarActorfromActorInfo))
  (bind _returnvalue_2 (Class|CombatInterface|GetCombatTarget(Message) _returnvalue))
  (bind _output_get (Variables|Default|SetProjectileTargetLocation (Transformation|GetActorLocation _returnvalue_2)))
  (Class|CombatInterface|UpdateFacingTarget(Message) _returnvalue _output_get)
  (bind _returnvalue_3 (Class|CombatInterface|GetAttackMontages(Message) (Ability|GetAvatarActorfromActorInfo)))
  (bind _output_get_2 (Variables|Default|SetTaggedAttackMontage (Class|AriaDamageGameplayAbility|GetRandomAttackMontage _returnvalue_3)))
  (Variables|Default|SetMontage (.AttackMontage (Utilities|Struct|BreakTaggedAttackMontage _output_get_2)))
  (Variables|Default|SetMontageTag (.AttackMontageTag (Utilities|Struct|BreakTaggedAttackMontage _output_get_2)))
  (Variables|Default|SetSocketTag (.AttackSocketTag (Utilities|Struct|BreakTaggedAttackMontage _output_get_2)))
  (Variables|Default|SetMontageImpactVFX (.AttackMontageImpactVFX (Utilities|Struct|BreakTaggedAttackMontage _output_get_2)))
  (Variables|Default|SetMontageImpactSFX (.AttackMontageImpactSFX (Utilities|Struct|BreakTaggedAttackMontage _output_get_2)))
  (|PlayMontageandWaitProxy "None" (Variables|Default|GetMontage) 1.0 "None" false 1.0 0.0 false
    (:then
      (Ability|Tasks|WaitGameplayEvent (Variables|Default|GetMontageTag) 0 true
        (:EventReceived
          (bind _returnvalue_4 (Class|CombatInterface|GetCombatSocketLocation(Message) (Ability|GetAvatarActorfromActorInfo) (Variables|Default|GetSocketTag)))
          (Variables|Default|SetCombatSocketLocation _returnvalue_4)
          (Variables|Default|SetProjectileDirection (Transformation|GetActorForwardVector (Ability|GetAvatarActorfromActorInfo))))))
    (:OnCompleted
      ;[1 1 1] This prevents the Animation from becoming locked up when the Enemies Attack gets interrupted.
      (Ability|EndAbility :!label _label))
    (:OnInterrupted
      (goto _label))
    (:OnCancelled
      (goto _label))))