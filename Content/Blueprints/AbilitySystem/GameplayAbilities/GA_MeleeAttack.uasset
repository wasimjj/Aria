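; GA_MeleeAttack is an enemy melee ability that turns the avatar toward its combat target and plays a random tagged attack montage.
; The montage's gameplay event triggers a small sphere query at the attack socket, ignoring "Enemy"-tagged actors.
; Non-friendly live actors in range take damage on the authority, and any hit fires the MeleeImpact gameplay cue.
; The ability ends after that check or when the montage completes or is interrupted.
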(event Ability|EventActivateAbility
  (bind _returnvalue (Ability|GetAvatarActorfromActorInfo))
  (Variables|Default|SetHasHitTarget false)
  ;[1 1 1] Get the Initial Target to Attack
  ; (Provided by the Ai Behavior Tree)
  (bind _returnvalue_2 (Class|CombatInterface|GetCombatTarget(Message) _returnvalue))
  (bind _output_get (Variables|Default|SetInitialCombatTarget _returnvalue_2))
  (Class|CombatInterface|UpdateFacingTarget(Message) _returnvalue (Transformation|GetActorLocation _output_get))
  (bind _returnvalue_3 (Class|CombatInterface|GetAttackMontages(Message) (Ability|GetAvatarActorfromActorInfo)))
  (bind _output_get_2 (Variables|Default|SetTaggedAttackMontage (Class|AriaDamageGameplayAbility|GetRandomAttackMontage _returnvalue_3)))
  (Variables|Default|SetMontage (.AttackMontage (Utilities|Struct|BreakTaggedAttackMontage _output_get_2)))
  (Variables|Default|SetMontageTag (.AttackMontageTag (Utilities|Struct|BreakTaggedAttackMontage _output_get_2)))
  (Variables|Default|SetSocketTag (.AttackSocketTag (Utilities|Struct|BreakTaggedAttackMontage _output_get_2)))
  (Variables|Default|SetMontageImpactVFX (.AttackMontageImpactVFX (Utilities|Struct|BreakTaggedAttackMontage _output_get_2)))
  (Variables|Default|SetMontageImpactSFX (.AttackMontageImpactSFX (Utilities|Struct|BreakTaggedAttackMontage _output_get_2)))
  (|PlayMontageandWaitProxy "None" (Variables|Default|GetMontage) 1.0 "None" false 1.0 0.0 false
    (:then
      ;[1 1 1] Calls back to the AN_MontageEvent > Event Tag specified in the Attack Animation Montage
      (Ability|Tasks|WaitGameplayEvent (Variables|Default|GetMontageTag) 0 true
        (:EventReceived
          (bind _returnvalue_4 (Class|CombatInterface|GetCombatSocketLocation(Message) (Ability|GetAvatarActorfromActorInfo) (Variables|Default|GetSocketTag)))
          (Variables|Default|SetCombatSocketLocation _returnvalue_4)
          (bind _outactors (Actor|GetAllActorswithTag "Enemy"))
          (bind _outoverlappingactors (Class|AriaAbilitySystemLibrary|GetLiveActorsWithinRadius self _outactors 45.0 (Variables|Default|GetCombatSocketLocation) false 1.0))
          (for _array_element _outoverlappingactors
            (bind _output_get_3 (Variables|Default|SetTargetActor _array_element))
            (if (Class|AriaAbilitySystemLibrary|IsNotFriend (Ability|GetAvatarActorfromActorInfo) _output_get_3)
              (Ability|HasAuthority
                (:True
                  (Class|AriaAbilitySystemLibrary|ApplyDamageEffect (Class|AriaDamageGameplayAbility|MakeAbilityModifierfromClassDefaults _output_get_3)))
                (:False
                  _))
              (Variables|Default|SetHasHitTarget true)))
          (if (Variables|Default|GetHasHitTarget)
            (Class|GameplayAbility|ExecuteGameplayCuewithParams "(TagName=\"GameplayCue.MeleeImpact\")" (Ability|GameplayCue|MakeGameplayCueParameters :AggregatedSourceTags (GameplayTags|MakeGameplayTagContainerfromTag (Variables|Default|GetMontageTag)) :Location (Variables|Default|GetCombatSocketLocation) :EffectCauser (Ability|GetAvatarActorfromActorInfo) :SourceObject (Variables|Default|GetInitialCombatTarget))))
          (Ability|EndAbility))))
    (:OnCompleted
      ;[1 1 1] This prevents the Animation from becoming locked up when the Enemies Attack gets interrupted.
      (Ability|EndAbility :!label _label))
    (:OnInterrupted
      (goto _label))
    (:OnCancelled
      (goto _label))))