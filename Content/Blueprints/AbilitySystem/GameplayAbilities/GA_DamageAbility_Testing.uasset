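; Test gameplay ability that prototypes a ground-targeted AoE cast, though no damage or effect spawning is connected.
; Activation shows a targeting reticle and waits for a press, then takes the impact point under the mouse and hides the reticle.
; It checks for the combat interface, turns the avatar to the target and plays the Firebolt montage.
; On the montage's gameplay event it queries the weapon socket, then ends after a short delay.
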(event Ability|EventActivateAbility
  (Utilities|FlowControl|Sequence
    (:then_0
      (Class|TargetingInterface|ShowAoETargetingReticle(Message) (Ability|GetAvatarActorfromActorInfo) 0 (Variables|Default|GetTargetingAreaRadius)))
    (:then_1
      (Ability|Tasks|WaitInputPress false
        (:OnPress
          (bind _datahandle (|TargetDataUnderMouse)
            (:ValidData
              (Variables|Default|SetImpactPoint (.ImpactPoint (Collision|BreakHitResult (Ability|TargetData|GetHitResultfromTargetData _datahandle))))
              (Class|TargetingInterface|HideAoETargetingReticle(Message) (Ability|GetAvatarActorfromActorInfo))
              (CallFunction|EnforceImplementsCombatInterface)
              (CallFunction|UpdateFacingTarget)
              (|PlayMontageandWaitProxy "None" "/Game/Assets/Characters/Aura/Animations/Abilities/AM_Cast_Firebolt.AM_Cast_Firebolt" 1.0 "None" false 1.0 0.0 false
                (:then
                  (Ability|Tasks|WaitGameplayEvent "(TagName=\"Event.Montage.Firebolt\")" 0 true
                    (:EventReceived
                      (Class|CombatInterface|GetCombatSocketLocation(Message) (Ability|GetAvatarActorfromActorInfo) (GameplayTags|MakeLiteralGameplayTag "(TagName=\"CombatSocket.Weapon\")"))
                      (Utilities|FlowControl|Delay 0.2)
                      (Ability|EndAbility))))))))))))

(fn UpdateFacingTarget
  (Class|CombatInterface|UpdateFacingTarget(Message) (Ability|GetAvatarActorfromActorInfo) (Variables|Default|GetImpactPoint)))

(fn EnforceImplementsCombatInterface
  ;[1 0.6096 0] Verify Implements the Combat Interface
  (if (not (Utilities|DoesObjectImplementInterface (Ability|GetAvatarActorfromActorInfo) "/Script/Aria.CombatInterface"))
    (Ability|EndAbility)))